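; Guard bot gameplay ability that shoots and damages the player on a hit.
; On activation it applies GE_Shoot to its owner, then waits for a single Shoot.Hit gameplay event.
; If the event's target has the Player actor tag, it applies GE_ShootDamage to that target.
; Any received hit forces the cooldown and ends the ability; without that event, the graph never ends it.
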(event `self.K2_ActivateAbility`
  (`self.BP_ApplyGameplayEffectToOwner` "/Game/HW_06/AI/Guard/BotAbilities/GE_Shoot.GE_Shoot_C")
  (bind (_asynctaskproxy _payload) (`AbilityTask_WaitGameplayEvent.WaitGameplayEvent` (struct :`TagName` "Event.Abilities.Shoot.Hit") null true)
    (:`EventReceived`
      (bind (_eventtag _instigator _target) (break `GameplayEventData` _payload))
      (if (`Actor.ActorHasTag` _target "Player")
        (`self.BP_ApplyGameplayEffectToTarget` (`AbilitySystemBlueprintLibrary.AbilityTargetDataFromActor` _target) "/Game/HW_06/AI/Guard/BotAbilities/GE_ShootDamage.GE_ShootDamage_C")
        (`self.K2_CommitAbilityCooldown` false true)
        (`self.K2_EndAbility`)
        (else
          (`self.K2_CommitAbilityCooldown` false true)
          (`self.K2_EndAbility`))))))